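; BossAI is a boss pawn that wanders to random reachable nearby points, pausing randomly between moves, and investigates noises.
; Sensed perception stimuli from NoiseMaker actors set IsInvestigating and send it to the stimulus location, then back to Roaming after a wait.
; IsInvestigating is never cleared, so that resumed roam stops after one move.
; Failed moves have no handling, and HandleHearingSense is an unused stub.
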(event `self.ReceiveBeginPlay`
  (`self.Roaming`))

(event `Roaming`
  (`|AIMoveTo` self (`NavigationSystemV1.K2_GetRandomReachablePointInRadius` (`SceneComponent.K2_GetComponentLocation` (`self.Mesh`)) 1500.0 null null) null
    (:`OnSuccess`
      (`KismetSystemLibrary.Delay` (`KismetMathLibrary.RandomFloatInRange` 0.0 5.0))
      (if (not (`self.isInvestigating`))
        (`self.Roaming`)))))

(event `self.AIPerception.OnTargetPerceptionUpdated`
  (params (Actor :type "Actor Object Reference") (Stimulus :type "AIStimulus Structure"))
  (bind (_age _expirationage _strength _stimuluslocation _receiverlocation _tag _bsuccessfullysensed) (break `AIStimulus` Stimulus))
  (cast `/Game/MyContents/Blueprints/NoiseMaker` Actor)
  (if _bsuccessfullysensed
    (set `self.isInvestigating` true)
    (`KismetSystemLibrary.PrintString` "Noise detected")
    (`|AIMoveTo` self _stimuluslocation null
      (:`OnSuccess`
        (`KismetSystemLibrary.Delay` 4.0)
        (`self.Roaming`)))))

(fn `Handle Hearing Sense`
  (params (Stimulus :type "AIStimulus Structure (by ref)"))
  (bind _returnvalue (`AIPerceptionSystem.GetSenseClassForStimulus` Stimulus))
  (if (== _returnvalue "/Script/AIModule.AISense_Hearing")
    _))

(fn `UserConstructionScript`)