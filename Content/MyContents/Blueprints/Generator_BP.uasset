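; Generator actor whose interaction is gated on whether the player has acquired a battery.
; Entering the Box enables or disables InteractionComponent from BP_GAD2010's BatteryAcquired flag, and leaving always re-enables it.
; The component's percent changes spin the PowerIcon and tilt the Switch through a clamped lerp.
; Nodes that would show a Battery_UI widget with mouse input are present but never run.
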(event `self.InteractionComponent.OnPercentChanged`
  (params (`New Percent` :type "Float (double-precision)"))
  ;[1 1 1] Animations
  (`SceneComponent.K2_SetRelativeRotation` (`self.PowerIcon`) (`KismetMathLibrary.MakeRotator` 0.0 0.0 (* `New Percent` 2000.0)) false false)
  (`SceneComponent.K2_SetRelativeRotation` (`self.Switch`) (`KismetMathLibrary.MakeRotator` (`KismetMathLibrary.Lerp` 40.0 140.0 (`KismetMathLibrary.MapRangeClamped` `New Percent` 0.0 1.0 0.0 1.0))) false false))

(event `self.Box.OnComponentBeginOverlap`
  (params (OverlappedComponent :type "PrimitiveComponent Object Reference") (OtherActor :type "Actor Object Reference") (OtherComp :type "PrimitiveComponent Object Reference") (OtherBodyIndex :type Integer) (bFromSweep :type Boolean) (SweepResult :type "HitResult Structure (by ref)"))
  ;[1 1 1] Condition Check
  (bind _asbp_gad2010 (cast `/Game/Base/Character/Blueprints/BP_GAD2010` OtherActor))
  (if (`/Game/Base/Character/Blueprints/BP_GAD2010.BatteryAcquired` _asbp_gad2010)
    (`/GAD2010Interaction/InteractionComponent.Set Enabled` (`self.InteractionComponent`) true)
    (else
      (`/GAD2010Interaction/InteractionComponent.Set Enabled` (`self.InteractionComponent`) false))))

(event `self.Box.OnComponentEndOverlap`
  (params (OverlappedComponent :type "PrimitiveComponent Object Reference") (OtherActor :type "Actor Object Reference") (OtherComp :type "PrimitiveComponent Object Reference") (OtherBodyIndex :type Integer))
  ;[1 1 1] Condition Check
  (cast `/Game/Base/Character/Blueprints/BP_GAD2010` OtherActor)
  (`/GAD2010Interaction/InteractionComponent.Set Enabled` (`self.InteractionComponent`) true))

(fn `UserConstructionScript`
  (`parent.UserConstructionScript`))