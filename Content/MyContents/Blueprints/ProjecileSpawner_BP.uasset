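; Spawner Blueprint that drops random projectile actors into a volume once the BP_GAD2010 actor enters its trigger box.
; Overlapping EntryBox sets InBox and starts a looping timer that fires SpawnProjectiles every few seconds, with no stop logic.
; Each firing spawns NumOfProjectiles actors, picking each class at random from ActorClass and each location at random within the SpawnRadius box bounds.
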(event `self.EntryBox.OnComponentBeginOverlap`
  (params (OverlappedComponent :type "PrimitiveComponent Object Reference") (OtherActor :type "Actor Object Reference") (OtherComp :type "PrimitiveComponent Object Reference") (OtherBodyIndex :type Integer) (bFromSweep :type Boolean) (SweepResult :type "HitResult Structure (by ref)"))
  ;[1 1 1] Spawn Projectiles
  (cast `/Game/Base/Character/Blueprints/BP_GAD2010` OtherActor)
  (set `self.InBox?` true)
  (`KismetSystemLibrary.K2_SetTimerDelegate` (delegate `SpawnProjectiles`) 4.0 true))

(event `SpawnProjectiles`
  (bind _spawnradius (`self.SpawnRadius`))
  ;[1 1 1] Spawn Projectiles
  (for _ (range (`self.NumOfProjectiles`))
    (`|SpawnActorFromClass` (`KismetArrayLibrary.Array_Random` (`self.ActorClass`)) (`KismetMathLibrary.Conv_VectorToTransform` (`KismetMathLibrary.RandomPointInBoundingBox` (`SceneComponent.K2_GetComponentLocation` _spawnradius) (`BoxComponent.GetScaledBoxExtent` _spawnradius))) "Undefined" "MultiplyWithRoot" null null)))

(fn `UserConstructionScript`)