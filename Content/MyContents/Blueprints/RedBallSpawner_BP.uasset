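; Spawner actor that drops red falling projectiles from random points inside its SpawnBox, up to three in total.
; Its SpawnBalls event spawns one projectile, increments the count and sets a flag that blocks further spawns.
; The flag clears when a red projectile ends overlap with the box, so the next SpawnBalls call can spawn again.
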(event `SpawnBalls`
  (bind _spawnbox (`self.SpawnBox`))
  (if (`self.IsSpawned`)
    _
    (elif (!= (`self.SpawnCount`) 3)
      (`|SpawnActorFromClass` "/Game/MyContents/Blueprints/RedFallingProjectiles_BP.RedFallingProjectiles_BP_C" (`KismetMathLibrary.Conv_VectorToTransform` (`KismetMathLibrary.RandomPointInBoundingBox` (`SceneComponent.K2_GetComponentLocation` _spawnbox) (`BoxComponent.GetScaledBoxExtent` _spawnbox))) "Undefined" "MultiplyWithRoot" null null)
      (`/Engine/EditorBlueprintResources/StandardMacros.IncrementInt` (`self.SpawnCount`)
        (:`  `
          (set `self.IsSpawned` true))))))

(event `self.SpawnBox.OnComponentEndOverlap`
  (params (OverlappedComponent :type "PrimitiveComponent Object Reference") (OtherActor :type "Actor Object Reference") (OtherComp :type "PrimitiveComponent Object Reference") (OtherBodyIndex :type Integer))
  (cast `/Game/MyContents/Blueprints/RedFallingProjectiles_BP` OtherActor)
  (set `self.IsSpawned` false))

(fn `UserConstructionScript`)