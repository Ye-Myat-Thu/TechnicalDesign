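; YellowBallReciever_BP is a receiver that collects falling projectiles and damages the boss once enough have arrived.
; When a FallingProjectiles_BP overlaps its Box, it destroys that projectile and increments YellowBallCount.
; When the count equals YellowBallMaxToDamage, it applies fixed damage to BossAI if that actor has the "Boss" tag.
; The counter is never reset in this graph, and all other events are empty.
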(event `self.Box.OnComponentBeginOverlap`
  (params (OverlappedComponent :type "PrimitiveComponent Object Reference") (OtherActor :type "Actor Object Reference") (OtherComp :type "PrimitiveComponent Object Reference") (OtherBodyIndex :type Integer) (bFromSweep :type Boolean) (SweepResult :type "HitResult Structure (by ref)"))
  (bind _bossai (`self.BossAI`))
  (bind _asfalling_projectiles_bp (cast `/Game/MyContents/Blueprints/FallingProjectiles_BP` OtherActor))
  (`self.K2_DestroyActor` _asfalling_projectiles_bp)
  (bind _result (`/Engine/EditorBlueprintResources/StandardMacros.IncrementInt` (`self.YellowBallCount`))
    (:`  `
      (if (== _result (`self.YellowBallMaxToDamage`))
        (if (`self.ActorHasTag` _bossai "Boss")
          (`GameplayStatics.ApplyDamage` _bossai 10.0))))))

(fn `UserConstructionScript`)