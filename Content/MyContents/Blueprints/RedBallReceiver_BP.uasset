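; RedBallReceiver_BP is a receiver that catches red falling projectiles and triggers damage once enough have landed.
; Its Box overlap casts to RedFallingProjectiles_BP, destroys the ball and increments RedBallCount.
; When the count equals RedBallMaxToDamage, it calls ApplyDamage on its AI controller, then deactivates the Box and reactivates it after a delay.
; The count is never reset in this Blueprint.
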(event `self.Box.OnComponentBeginOverlap`
  (params (OverlappedComponent :type "PrimitiveComponent Object Reference") (OtherActor :type "Actor Object Reference") (OtherComp :type "PrimitiveComponent Object Reference") (OtherBodyIndex :type Integer) (bFromSweep :type Boolean) (SweepResult :type "HitResult Structure (by ref)"))
  (bind _asred_falling_projectiles_bp (cast `/Game/MyContents/Blueprints/RedFallingProjectiles_BP` OtherActor))
  (`self.K2_DestroyActor` _asred_falling_projectiles_bp)
  (bind _result (`/Engine/EditorBlueprintResources/StandardMacros.IncrementInt` (`self.RedBallCount`))
    (:`  `
      (if (== _result (`self.RedBallMaxToDamage`))
        (`GameplayStatics.ApplyDamage` (`AIBlueprintHelperLibrary.GetAIController` null))
        (`ActorComponent.Deactivate` (`self.Box`))
        (`KismetSystemLibrary.Delay` 10.0)
        (`ActorComponent.Activate` (`self.Box`) false)))))

(fn `UserConstructionScript`)