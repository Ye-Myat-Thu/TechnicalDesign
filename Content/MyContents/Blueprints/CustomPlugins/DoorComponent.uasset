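; DoorComponent is a component that opens and closes its owning actor as a lifting door by changing its height.
; LiftDoor acts only while InBox is true, and CloseDoor only while it is false.
; Each sets Alpha to an endpoint and moves the owner to NewX, NewY and a Lerp between InitialZ and NewZ, so the door snaps rather than animates.
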(event `Lift Door`
  (if (`self.inBox?`)
    (bind _output_get (set `self.Alpha` 1.0))
    (`Actor.K2_SetActorLocation` (`self.GetOwner`) (`KismetMathLibrary.MakeVector` (`self.New X`) (`self.New Y`) (`KismetMathLibrary.Lerp` (`self.Initial Z`) (`self.New Z`) _output_get)) false false)))

(event `Close Door`
  (if (not (`self.inBox?`))
    (bind _output_get (set `self.Alpha` 0.0))
    (`Actor.K2_SetActorLocation` (`self.GetOwner`) (`KismetMathLibrary.MakeVector` (`self.New X`) (`self.New Y`) (`KismetMathLibrary.Lerp` (`self.Initial Z`) (`self.New Z`) _output_get)) false false)))