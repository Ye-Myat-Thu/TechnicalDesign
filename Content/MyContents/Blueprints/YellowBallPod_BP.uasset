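; YellowBallPod_BP is a collector pod that catches falling projectiles and tracks how full it is.
; When a FallingProjectiles_BP overlaps PodBox, it destroys that projectile and increments YellowBallCount, with no colour check in this graph.
; When the count reaches YellowMaxBall, it sets YellowPodFull, destroys PodBox to stop further catches and switches the mesh to Silver_Metallic.
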(event `self.PodBox.OnComponentBeginOverlap`
  (params (OverlappedComponent :type "PrimitiveComponent Object Reference") (OtherActor :type "Actor Object Reference") (OtherComp :type "PrimitiveComponent Object Reference") (OtherBodyIndex :type Integer) (bFromSweep :type Boolean) (SweepResult :type "HitResult Structure (by ref)"))
  (bind _asfalling_projectiles_bp (cast `/Game/MyContents/Blueprints/FallingProjectiles_BP` OtherActor))
  (`self.K2_DestroyActor` _asfalling_projectiles_bp)
  (bind _result (`/Engine/EditorBlueprintResources/StandardMacros.IncrementInt` (`self.YellowBallCount`))
    (:`  `
      (if (== _result (`self.YellowMaxBall`))
        (set `self.Yellow Pod Full` true)
        (`ActorComponent.K2_DestroyComponent` (`self.PodBox`))
        (`PrimitiveComponent.SetMaterial` (`self.StaticMesh`) 0 "/Game/MyContents/MyMeshes/Textures/Silver_Metallic.Silver_Metallic")))))

(fn `UserConstructionScript`)