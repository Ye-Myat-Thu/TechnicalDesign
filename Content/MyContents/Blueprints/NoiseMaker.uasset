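; NoiseMaker is an interactable lever actor that emits a noise at its own location when used.
; A short interaction on its InteractionComponent calls MakeNoise on the NoiseComponent, prints the location and snaps the Lever to a pulled rotation.
; The IsEnabled flag blocks reuse during a ten-second delay, after which the lever resets and can be used again.
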(event `self.InteractionComponent.OnShortInteraction`
  (params (Instigator :type "Actor Object Reference"))
  (bind _returnvalue (`self.K2_GetActorLocation`))
  (if (not (`self.isEnabled`))
    (`/Game/MyContents/Blueprints/AI_NoiseEmitter_Plugin/NoiseComponent.Make Noise` (`self.NoiseComponent`) _returnvalue)
    (`KismetSystemLibrary.PrintString` (`KismetStringLibrary.Conv_VectorToString` _returnvalue))
    (set `self.isEnabled` true)
    (`SceneComponent.K2_SetRelativeRotation` (`self.Lever`) (struct :`Roll` -90.0) false false)
    (`KismetSystemLibrary.Delay` 10.0)
    (`SceneComponent.K2_SetRelativeRotation` (`self.Lever`) (struct) false false)
    (set `self.isEnabled` false)))

(fn `UserConstructionScript`)