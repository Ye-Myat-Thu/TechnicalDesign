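; CollapsingFloor_BP is a floor that collapses under a BP_GAD2010 actor once the yellow and red pod challenge is complete.
; Tick polls both pods and, while both are full, sets IsValid and reapplies a glow material to the ring, which starts as a hologram.
; Overlapping the box while valid turns on floor physics, then destroys the whole actor after a short delay.
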(event `self.ReceiveTick`
  (params (DeltaSeconds :type "Float (single-precision)"))
  (if (and (`/Game/MyContents/Blueprints/YellowBallPod_BP.Yellow Pod Full` (`self.YellowPod`)) (`/Game/MyContents/Blueprints/RedBallPod_BP.Red Pod Full` (`self.RedPod`)))
    (set `self.IsValid?` true)
    (`self.IsValid`)))

(event `self.ReceiveBeginPlay`
  ;[1 1 1] Initial Material of the ring, challenge still ongoing
  (if (not (`self.IsValid?`))
    (`PrimitiveComponent.SetMaterial` (`self.Ring`) 0 "/Game/MyContents/MyMeshes/Textures/Hologram.Hologram")))

(event `IsValid`
  ;[1 1 1] Initial Material of the ring, challenge still ongoing
  (`PrimitiveComponent.SetMaterial` (`self.Ring`) 0 "/Game/PolygonPrototype/Materials/Mat_Polygon_Prototype_Glow_Ring_FX.Mat_Polygon_Prototype_Glow_Ring_FX"))

(event `self.Box.OnComponentBeginOverlap`
  (params (OverlappedComponent :type "PrimitiveComponent Object Reference") (OtherActor :type "Actor Object Reference") (OtherComp :type "PrimitiveComponent Object Reference") (OtherBodyIndex :type Integer) (bFromSweep :type Boolean) (SweepResult :type "HitResult Structure (by ref)"))
  ;[1 1 1] Collapsed when overlapped
  (cast `/Game/Base/Character/Blueprints/BP_GAD2010` OtherActor)
  (if (`self.IsValid?`)
    (`PrimitiveComponent.SetSimulatePhysics` (`self.Floor`) true)
    (`KismetSystemLibrary.Delay` 0.2)
    (`self.K2_DestroyActor`)))

(fn `UserConstructionScript`)