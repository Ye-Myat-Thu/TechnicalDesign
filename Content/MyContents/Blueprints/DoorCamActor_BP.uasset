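; DoorCamActor_BP is a trigger actor that switches the player's view to another camera, apparently for a door area.
; When a BP_GAD2010 begins overlapping Trigger, its player controller, reached through PlayerState, sets the view target to CamActor.
; When the overlap ends, that controller's view target returns to player character 0, whichever player left the trigger.
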(event `self.Trigger.OnComponentBeginOverlap`
  (params (OverlappedComponent :type "PrimitiveComponent Object Reference") (OtherActor :type "Actor Object Reference") (OtherComp :type "PrimitiveComponent Object Reference") (OtherBodyIndex :type Integer) (bFromSweep :type Boolean) (SweepResult :type "HitResult Structure (by ref)"))
  (bind _asbp_gad2010 (cast `/Game/Base/Character/Blueprints/BP_GAD2010` OtherActor))
  (`PlayerController.SetViewTargetWithBlend` (`PlayerState.GetPlayerController` (`Pawn.PlayerState` _asbp_gad2010)) (`self.Cam Actor`) 0.0 "VTBlend_Linear" 0.0 false))

(event `self.Trigger.OnComponentEndOverlap`
  (params (OverlappedComponent :type "PrimitiveComponent Object Reference") (OtherActor :type "Actor Object Reference") (OtherComp :type "PrimitiveComponent Object Reference") (OtherBodyIndex :type Integer))
  (bind _asbp_gad2010 (cast `/Game/Base/Character/Blueprints/BP_GAD2010` OtherActor))
  (`PlayerController.SetViewTargetWithBlend` (`PlayerState.GetPlayerController` (`Pawn.PlayerState` _asbp_gad2010)) (`GameplayStatics.GetPlayerCharacter` 0) 0.0 "VTBlend_Linear" 0.0 false))

(fn `UserConstructionScript`)