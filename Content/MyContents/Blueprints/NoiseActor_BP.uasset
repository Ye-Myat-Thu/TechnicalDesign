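; NoiseActor_BP is a pressure button actor that emits a noise when the BP_GAD2010 actor steps into its box trigger.
; On overlap it lowers the Button component slightly and calls NoiseMaker on its MakeNoiseComponent at the actor's location.
; A short delay then returns the button to its resting height, giving a simple press animation without a timeline.
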(event `self.Box.OnComponentBeginOverlap`
  (params (OverlappedComponent :type "PrimitiveComponent Object Reference") (OtherActor :type "Actor Object Reference") (OtherComp :type "PrimitiveComponent Object Reference") (OtherBodyIndex :type Integer) (bFromSweep :type Boolean) (SweepResult :type "HitResult Structure (by ref)"))
  (cast `/Game/Base/Character/Blueprints/BP_GAD2010` OtherActor)
  (`self.SetAnimation`)
  (`/AIPerception/MakeNoiseComponent.NoiseMaker` (`self.MakeNoiseComponent`) (`self.K2_GetActorLocation`))
  (`self.ResetAnimation`))

(event `SetAnimation`
  (`SceneComponent.K2_SetRelativeLocation` (`self.Button`) (0.0 0.0 -3.75) false false))

(event `ResetAnimation`
  (`KismetSystemLibrary.Delay` 0.2)
  (`SceneComponent.K2_SetRelativeLocation` (`self.Button`) (0.0 0.0 -0.0) false false))

(fn `UserConstructionScript`)