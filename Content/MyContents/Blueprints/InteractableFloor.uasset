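; InteractableFloor is an actor that moves vertically in response to another actor's interaction progress.
; On BeginPlay it binds to the watched InteractiveActorToWatch's InteractionComponent percent-changed event and snaps to a hardcoded raised position.
; Each percent change is remapped between configurable min and max percentages and lerps only its height, lowering the floor as progress rises.
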(event `self.ReceiveBeginPlay`
  (bind _output_get (set `self.Interactive Actor To Watch` (`self.Interactive Actor To Watch`)))
  (add `/GAD2010Interaction/InteractionComponent.OnPercentChanged` (`/GAD2010Interaction/InteractiveActorBase.InteractionComponent` _output_get) (delegate `FloorAlignment`))
  (`self.K2_SetActorLocation` (950.0 150.0 80.0)))

(event `FloorAlignment`
  (params (`New Percent` :type "Float (double-precision)"))
  (`self.K2_SetActorLocation` (`KismetMathLibrary.MakeVector` 950.0 150.0 (`KismetMathLibrary.Lerp` 80.0 0.0 (`KismetMathLibrary.MapRangeClamped` `New Percent` (`self.Min Percentge`) (`self.Max Percentage`) 0.0 1.0)))))

(fn `UserConstructionScript`)