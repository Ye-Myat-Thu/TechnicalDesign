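; EncounterGameMode is a game mode that handles player start selection and checkpoint respawning.
; Respawning teleports the first player's pawn to the stored checkpoint and calls OnRespawn, or opens the EncounterHub level if no checkpoint is valid.
; In the hub, ChoosePlayerStart picks the first actor tagged "Skip" when the game instance's SkipTitle flag is set, and otherwise falls back to the parent selection.
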(fn `AttemptRespawn`
  ;[1 1 1] Move the character to a checkpoint, if possible. Go to the hub if not.
  (bind _checkpoint (`self.Checkpoint`)
    (:`then`
      (`self.K2_TeleportTo` (`GameplayStatics.GetPlayerPawn` 0) (`self.K2_GetActorLocation` _checkpoint) (`self.K2_GetActorRotation` _checkpoint))
      (`self.OnRespawn`))
    (:`else`
      (`GameplayStatics.OpenLevelBySoftObjectPtr` "/Game/Base/Maps/EncounterHub.EncounterHub"))))

(fn `ChoosePlayerStart`
  (params (Player :type "Controller Object Reference"))
  (returns (ReturnValue :type "Actor Object Reference"))
  (bind _returnvalue (`GameplayStatics.GetCurrentLevelName` true))
  (if (`KismetStringLibrary.EqualEqual_StrStr` _returnvalue "EncounterHub")
    (bind _asencounter_game_instance (cast `/Game/Base/Blueprints/EncounterGameInstance` (`GameplayStatics.GetGameInstance`)))
    (if (`/Game/Base/Blueprints/EncounterGameInstance.SkipTitle` _asencounter_game_instance)
      (bind _outactors (`GameplayStatics.GetAllActorsWithTag` "Skip"))
      (return (`|GetArrayItem` _outactors))
      (else
        _)))
  (bind _returnvalue_2 (`parent.ChoosePlayerStart` (`local.Player`)))
  (return _returnvalue_2))

(fn `SetCheckpoint`
  (params (`New Checkpoint` :type "Actor Object Reference"))
  ;[1 1 1] Used to set in-level checkpoints
  (set `self.Checkpoint` `New Checkpoint`))

(fn `UserConstructionScript`)