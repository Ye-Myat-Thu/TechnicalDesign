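; LevelLoader is an interactable actor that sends the player to another level, marked by a floating icon.
; When the long interaction reaches a specific phase, it creates a ScreenFade widget, plays a fade, waits for its duration, then opens LevelToLoad by object reference.
; Every tick, the icon spins and bobs on a sine wave driven by game time.
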(event `self.InteractionComponent.OnLongInteraction`
  (params (Instigator :type "Actor Object Reference") (Phase :type "/GAD2010Interaction/InteractionPhase Enum" :default "NewEnumerator0") (Delta :type "Float (double-precision)"))
  (bind _fadeduration (`self.FadeDuration`))
  ;[1 1 1] Loads the selected level after a long interaction.
  (if (`|EnumEquality` Phase "NewEnumerator2")
    (bind _returnvalue (`|CreateWidget` "/Game/Base/Widgets/ScreenFade.ScreenFade_C"))
    (`UserWidget.AddToViewport` _returnvalue 0)
    (`/Game/Base/Widgets/ScreenFade.PlayFade` _returnvalue _fadeduration false)
    (`KismetSystemLibrary.Delay` _fadeduration)
    (`GameplayStatics.OpenLevelBySoftObjectPtr` (`self.LevelToLoad`))))

(event `self.ReceiveTick`
  (params (DeltaSeconds :type "Float (single-precision)"))
  (bind _returnvalue (`KismetSystemLibrary.GetGameTimeInSeconds`))
  (`SceneComponent.K2_SetRelativeLocationAndRotation` (`self.Icon`) (`KismetMathLibrary.MakeVector` 0.0 0.0 (+ 100.0 (* 10.0 (`KismetMathLibrary.Sin` _returnvalue)))) (`KismetMathLibrary.MakeRotator` 0.0 -20.0 (* _returnvalue 60.0)) false false))

(fn `UserConstructionScript`)